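; YeetInstance, apparently the game instance, holds Yeet Yourself's world progress, movement and ability keybinds, and mouse sensitivity.
; SetNewWorldInt only ever raises the world index and does not save it.
; SaveKeybindsAndSens writes controls and sensitivity to SaveSlot, while ResetGame clears world progress and writes it there.
; Both build a fresh Saved object rather than loading the existing one, so each overwrites the other's fields with class defaults.
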(fn `ResetGame`
  (locals (SaveRef :type "/Game/YeetYourself/Blueprints/Saved Object Reference"))
  (bind _returnvalue (`GameplayStatics.CreateSaveGameObject` "/Game/YeetYourself/Blueprints/Saved.Saved_C"))
  (bind _output_get (set `local.SaveRef` _returnvalue))
  (bind _output_get_2 (set `self.WorldInt` 0))
  (set `/Game/YeetYourself/Blueprints/Saved.WorldInt_Save` _output_get_2 _output_get)
  (bind _output_get_3 (set `self.World2` false))
  (set `/Game/YeetYourself/Blueprints/Saved.World2_Save` _output_get_3 _output_get)
  (bind _output_get_4 (set `self.World3` false))
  (set `/Game/YeetYourself/Blueprints/Saved.World3_Save` _output_get_4 _output_get)
  (`GameplayStatics.SaveGameToSlot` _returnvalue "SaveSlot"))

(fn `SaveKeybindsAndSens`
  (locals (SaveRef :type "/Game/YeetYourself/Blueprints/Saved Object Reference"))
  (bind _returnvalue (`GameplayStatics.CreateSaveGameObject` "/Game/YeetYourself/Blueprints/Saved.Saved_C"))
  (bind _output_get (set `local.SaveRef` _returnvalue))
  (set `/Game/YeetYourself/Blueprints/Saved.Foward_Save` (`self.Forward`) _output_get)
  (set `/Game/YeetYourself/Blueprints/Saved.Backward_Save` (`self.Backward`) _output_get)
  (set `/Game/YeetYourself/Blueprints/Saved.Left_Save` (`self.Left`) _output_get)
  (set `/Game/YeetYourself/Blueprints/Saved.Right_Save` (`self.Right`) _output_get)
  (set `/Game/YeetYourself/Blueprints/Saved.MomentumCancel_Save` (`self.MomentumCancel`) _output_get)
  (set `/Game/YeetYourself/Blueprints/Saved.Yoink_Save` (`self.Yoink`) _output_get)
  (set `/Game/YeetYourself/Blueprints/Saved.Yeet_Save` (`self.Yeet`) _output_get)
  (set `/Game/YeetYourself/Blueprints/Saved.Jump_Save` (`self.Jump`) _output_get)
  (set `/Game/YeetYourself/Blueprints/Saved.MouseSensitivity_Save` (`self.Mouse Sensitivity`) _output_get)
  (`GameplayStatics.SaveGameToSlot` _returnvalue "SaveSlot"))

(fn `SetNewWorldInt`
  (params (NewWorldInt :type Integer))
  (`/Engine/EditorBlueprintResources/StandardMacros.CompareInt` NewWorldInt (`self.WorldInt`)
    (:`>`
      (set `self.WorldInt` NewWorldInt))))